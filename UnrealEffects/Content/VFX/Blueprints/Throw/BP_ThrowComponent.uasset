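; Actor component that lets the third-person character aim and throw bombs.
; Aiming spawns a BP_Bomb on the hand socket, plays the throw montage and shows the HUD scope; cancelling switches the montage to its Static section.
; Throwing detaches the bomb and launches it with a physics impulse blending actor and camera forward.
; ABP_Throwing receives the aim state, while ResetShoot re-enables throwing and respawns a bomb if still aiming.
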(event `self.ReceiveBeginPlay`
  (bind _asbp_third_person_character (cast `/Game/ThirdPerson/Blueprints/BP_ThirdPersonCharacter` (`self.GetOwner`)))
  (set `self.Owner` _asbp_third_person_character)
  (bind _asabp_throwing (cast `/Game/VFX/Animation/ABP_Throwing` (`SkeletalMeshComponent.GetAnimInstance` (`Character.Mesh` _asbp_third_person_character))))
  (set `self.Animation Blueprint` _asabp_throwing)
  (bind _asbp_hud (cast `/Game/VFX/Blueprints/Throw/BP_HUD` (`PlayerController.GetHUD` (`GameplayStatics.GetPlayerController` 0))))
  (set `self.HUD` _asbp_hud))

(fn `Aim`
  (if (not (`self.Aiming`))
    (`self.SpawnBomb`)
    (`/Game/VFX/Blueprints/Throw/BP_HUD.Show Scope` (`self.HUD`) true)
    (`Character.PlayAnimMontage` (`self.Owner`) "/Game/VFX/Animation/AM_Throw.AM_Throw" 1.0 "Init")
    (set `self.Aiming` true)
    (set `/Game/VFX/Animation/ABP_Throwing.IsAiming` true (`self.Animation Blueprint`))))

(fn `Cancel Aiming`
  (bind _returnvalue (`SkeletalMeshComponent.GetAnimInstance` (`Character.Mesh` (`self.Owner`))))
  (bind _returnvalue_2 (`AnimInstance.GetCurrentActiveMontage` _returnvalue))
  (if (`self.Aiming`)
    (set `/Game/VFX/Animation/ABP_Throwing.CancelledThrowing` true (`self.Animation Blueprint`))
    (`self.Disband Aim` false)
    (`AnimInstance.Montage_SetNextSection` _returnvalue (`AnimInstance.Montage_GetCurrentSection` _returnvalue _returnvalue_2) "Static" _returnvalue_2)
    (`/Game/VFX/Blueprints/Throw/BP_HUD.Show Scope` (`self.HUD`) false)))

(fn `DeleteBomb`
  (bind _thrown_item (`self.Thrown Item`)
    (:`then`
      (`Actor.K2_DestroyActor` _thrown_item)
      (set `self.Thrown Item` null))
    (:`else`)))

(fn `Disband Aim`
  (params (`Keep Aiming?` :type Boolean))
  (set `self.Aiming` `Keep Aiming?`)
  (set `/Game/VFX/Animation/ABP_Throwing.IsAiming` false (`self.Animation Blueprint`)))

(fn `Reset Shoot`
  (set `self.Can Shoot` true)
  (if (`self.Aiming`)
    (set `/Game/VFX/Animation/ABP_Throwing.IsAiming` true (`self.Animation Blueprint`))
    (`self.SpawnBomb`)))

(fn `setActor`
  (params (`Throwing Actor` :type "StaticMeshActor Object Reference"))
  ;[1 1 1] En un juego complejo aquí habría comprobaciones de tipo o enums y tal
)

(fn `SpawnBomb`
  (bind _returnvalue (`|SpawnActorFromClass` "/Game/VFX/Blueprints/Throw/BP_Bomb.BP_Bomb_C" (`KismetMathLibrary.MakeTransform` (0.0 0.0 0.0)) "AdjustIfPossibleButAlwaysSpawn" "MultiplyWithRoot" null null))
  (bind _output_get (set `self.Thrown Item` _returnvalue))
  (`PrimitiveComponent.SetCollisionEnabled` (`/Game/VFX/Blueprints/Throw/BP_Bomb.Sphere` _output_get) "NoCollision")
  (`Actor.K2_AttachToComponent` _output_get (`Character.Mesh` (`self.Owner`)) "Weapon_r" "KeepRelative" "KeepRelative" "KeepRelative" true))

(fn `Throw`
  (bind _owner (`self.Owner`))
  (if (and (`self.Aiming`) (`self.Can Shoot`))
    (set `self.Can Shoot` false)
    (bind _thrown_item (`self.Thrown Item`)
      (:`then`
        (`Actor.K2_DetachFromActor` _thrown_item "KeepWorld" "KeepWorld" "KeepWorld")
        (bind _sphere (`/Game/VFX/Blueprints/Throw/BP_Bomb.Sphere` _thrown_item))
        (`PrimitiveComponent.SetSimulatePhysics` _sphere true)
        (`PrimitiveComponent.SetCollisionEnabled` _sphere "QueryAndPhysics")
        (`PrimitiveComponent.AddImpulse` _sphere (* (`self.Strength`) (`KismetMathLibrary.Normal` (+ (`Actor.GetActorForwardVector` _owner) (`SceneComponent.GetForwardVector` (`/Game/ThirdPerson/Blueprints/BP_ThirdPersonCharacter.FollowCamera` _owner))))) "None" false)
        (`/Game/VFX/Blueprints/Throw/BP_Bomb.Thrown` (`self.Thrown Item`))
        (set `/Game/VFX/Animation/ABP_Throwing.CancelledThrowing` false (`self.Animation Blueprint`))
        (`self.Disband Aim` true)
        (set `self.Thrown Item` null))
      (:`else`))))