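; Playground actor that paints a brush into a render target at the surface UV directly beneath it.
; BeginPlay creates a dynamic instance of the Brush material and clears the render target to black.
; Each Tick, a short downward complex trace finds the hit UV, feeds it to the material's U/V parameters, and draws that material into the target without clearing.
; Trace debug drawing and a Print String remain active.
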(event `self.ReceiveBeginPlay`
  (`parent.ReceiveBeginPlay`)
  (bind _brush (`self.Brush`)
    (:`then`
      (bind _returnvalue (`KismetMaterialLibrary.CreateDynamicMaterialInstance` _brush))
      (set `self.RenderTargetMaterial` _returnvalue)
      (`KismetRenderingLibrary.ClearRenderTarget2D` (`self.Render Target`)))
    (:`else`)))

(event `self.ReceiveTick`
  (params (DeltaSeconds :type "Float (single-precision)"))
  (bind _returnvalue (`self.K2_GetActorLocation`))
  (bind _rendertargetmaterial (`self.RenderTargetMaterial`))
  (bind _outhit (`KismetSystemLibrary.LineTraceSingle` :`Start` _returnvalue :`End` (+ _returnvalue (0.0 0.0 -200.0)) :`TraceChannel` "TraceTypeQuery3" :`bTraceComplex` true :`DrawDebugType` "ForDuration"))
  (bind _uv (`GameplayStatics.FindCollisionUV` _outhit))
  (`MaterialInstanceDynamic.SetScalarParameterValue` _rendertargetmaterial "U" (`KismetMathLibrary.BreakVector2D` _uv))
  (`MaterialInstanceDynamic.SetScalarParameterValue` _rendertargetmaterial "V" (`.Y` (`KismetMathLibrary.BreakVector2D` _uv)))
  (`KismetRenderingLibrary.DrawMaterialToRenderTarget` (`self.Render Target`) (`self.RenderTargetMaterial`))
  (`KismetSystemLibrary.PrintString` "Hello"))

(fn `UserConstructionScript`
  (`parent.UserConstructionScript`))