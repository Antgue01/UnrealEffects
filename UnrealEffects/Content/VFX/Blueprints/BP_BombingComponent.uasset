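; Actor component that lets a Character owner hold a bomb, with functions to spawn and delete it.
; BeginPlay caches the owning Character's mesh, which serves as the attach parent.
; SpawnBomb creates a bomb actor, disables its sphere collision and attaches it to the Weapon_r socket.
; DeleteBomb destroys the stored bomb if it is valid and clears the reference.
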(event `self.ReceiveBeginPlay`
  (bind _ascharacter (cast `Character` (`self.GetOwner`)))
  (set `self.Mesh` (`Character.Mesh` _ascharacter)))

(fn `DeleteBomb`
  (bind _bomb (`self.Bomb`)
    (:`then`
      (`Actor.K2_DestroyActor` _bomb)
      (set `self.Bomb` null))
    (:`else`)))

(fn `SpawnBomb`
  (bind _returnvalue (`|SpawnActorFromClass` "/Game/VFX/Blueprints/BP_Bomb.BP_Bomb_C" (`KismetMathLibrary.MakeTransform` (0.0 0.0 0.0)) "AdjustIfPossibleButAlwaysSpawn" "MultiplyWithRoot" null null))
  (`PrimitiveComponent.SetCollisionEnabled` (`/Game/VFX/Blueprints/BP_Bomb.Sphere` _returnvalue) "NoCollision")
  (bind _output_get (set `self.Bomb` _returnvalue))
  (`Actor.K2_AttachToComponent` _output_get (`self.Mesh`) "Weapon_r" "KeepRelative" "KeepRelative" "KeepRelative" true))